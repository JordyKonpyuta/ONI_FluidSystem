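; BP_Liquid is a liquid particle actor that simulates fluids of differing densities settling into layers.
; On BeginPlay it takes a random DT_LiquidTypes row for density and color, tints a dynamic material, and starts a looping timer.
; VerifyNeighbors line-traces down and along ±Y, stepping the actor down or sideways by fixed offsets.
; When it hits another BP_Liquid, the less dense one is teleported upward, approximating buoyancy without physics.
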(event `self.ReceiveBeginPlay`
  (`self.InitLiquid`)
  (bind _returnvalue (`KismetSystemLibrary.K2_SetTimerDelegate` (`|CreateDelegate` :!event `VerifyNeighbors`) 0.08 true))
  (set `self.TimerRef` _returnvalue))

(event `VerifyNeighbors`
  (bind _returnvalue (`self.K2_GetActorLocation`))
  (bind _returnvalue_2 (`self.K2_GetActorLocation`))
  (bind _returnvalue_3 (`self.K2_GetActorLocation`))
  (`|ExecutionSequence`
    (:`then_0`
      (bind (_outhit _returnvalue_4) (`KismetSystemLibrary.LineTraceSingleForObjects` _returnvalue (- _returnvalue (0.0 0.0 200.0)) (`|MakeArray` "ObjectTypeQuery7" "ObjectTypeQuery8" :!type "EObjectTypeQuery Enum")))
      (if _returnvalue_4
        (bind _asbp_liquid (cast `/Game/BP_Liquid` (`.HitActor` (`GameplayStatics.BreakHitResult` _outhit))))
        (if (< (`/Game/BP_Liquid.Density` _asbp_liquid) (`self.Density`))
          (`self.K2_SetActorLocation` _asbp_liquid (+ (`self.K2_GetActorLocation` _asbp_liquid) (0.0 0.0 300.0)) false false)
          (elif (> (`/Game/BP_Liquid.Density` _asbp_liquid) (`self.Density`))
            (`self.K2_SetActorLocation` (+ (`self.K2_GetActorLocation`) (0.0 0.0 300.0)))))
        (else
          (`self.K2_SetActorLocation` (- (`self.K2_GetActorLocation`) (0.0 0.0 40.0))))))
    (:`then_1`
      (bind (_outhit_2 _returnvalue_5) (`KismetSystemLibrary.LineTraceSingleForObjects` _returnvalue_2 (+ _returnvalue_2 (0.0 150.0 0.0)) (`|MakeArray` "ObjectTypeQuery7" "ObjectTypeQuery8" :!type "EObjectTypeQuery Enum")))
      (bind (_outhit_3 _returnvalue_6) (`KismetSystemLibrary.LineTraceSingleForObjects` _returnvalue_3 (- _returnvalue_3 (0.0 150.0 0.0)) (`|MakeArray` "ObjectTypeQuery7" "ObjectTypeQuery8" :!type "EObjectTypeQuery Enum")))
      (if (and _returnvalue_6 _returnvalue_5)
        (bind _asbp_liquid_2 (cast `/Game/BP_Liquid` (`.HitActor` (`GameplayStatics.BreakHitResult` _outhit_3))))
        (if (< (`/Game/BP_Liquid.Density` _asbp_liquid_2) (`self.Density`))
          (`self.K2_SetActorLocation` _asbp_liquid_2 (+ (`self.K2_GetActorLocation`) (0.0 0.0 300.0)) false false)
          (elif (> (`/Game/BP_Liquid.Density` _asbp_liquid_2) (`self.Density`))
            (`self.K2_SetActorLocation` (+ (`self.K2_GetActorLocation`) (0.0 0.0 300.0)))))
        (elif (and _returnvalue_6 (not _returnvalue_5))
          (`self.K2_SetActorLocation` (+ (`self.K2_GetActorLocation`) (0.0 40.0 0.0)))
          (bind _asbp_liquid_3 (cast `/Game/BP_Liquid` (`.HitActor` (`GameplayStatics.BreakHitResult` _outhit_3))))
          (if (< (`/Game/BP_Liquid.Density` _asbp_liquid_3) (`self.Density`))
            (`self.K2_SetActorLocation` _asbp_liquid_3 (+ (`self.K2_GetActorLocation`) (0.0 0.0 300.0)) false false)
            (elif (> (`/Game/BP_Liquid.Density` _asbp_liquid_3) (`self.Density`))
              (`self.K2_SetActorLocation` (+ (`self.K2_GetActorLocation`) (0.0 0.0 300.0)))))
          (else
            (`self.K2_SetActorLocation` (- (`self.K2_GetActorLocation`) (0.0 40.0 0.0)))
            (bind _asbp_liquid_4 (cast `/Game/BP_Liquid` (`.HitActor` (`GameplayStatics.BreakHitResult` _outhit_3))))
            (if (< (`/Game/BP_Liquid.Density` _asbp_liquid_4) (`self.Density`))
              (`self.K2_SetActorLocation` _asbp_liquid_4 (+ (`self.K2_GetActorLocation`) (0.0 0.0 300.0)) false false)
              (elif (> (`/Game/BP_Liquid.Density` _asbp_liquid_4) (`self.Density`))
                (`self.K2_SetActorLocation` (+ (`self.K2_GetActorLocation`) (0.0 0.0 300.0)))))))))))

(fn `InitLiquid`
  (bind _returnvalue (`|GetDataTableRow` "/Game/DT_LiquidTypes.DT_LiquidTypes" (`KismetStringLibrary.Conv_StringToName` (`KismetStringLibrary.Conv_IntToString` (`KismetMathLibrary.RandomIntegerInRange` 0 3))))
    (:`then`
      (bind (_name _density _color) (break `/Game/S_LiquidTypes` _returnvalue))
      (set `self.Density` _density)
      (bind _returnvalue_2 (`KismetMaterialLibrary.CreateDynamicMaterialInstance` "/Game/MI_Fluid.MI_Fluid"))
      (bind _output_get (set `self.Material` _returnvalue_2))
      (`MaterialInstanceDynamic.SetVectorParameterValue` _returnvalue_2 "Color" _color)
      (`MaterialInstanceDynamic.SetVectorParameterValue` _output_get "Color" _color)
      (`PrimitiveComponent.SetMaterial` (`self.StaticMesh`) 0 (`self.Material`)))))

(fn `UserConstructionScript`)